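; Enemy character pawn that shows a world-space sight meter while detecting and signals its AI to start or stop chasing.
; StartDetection reveals and fills the WD_EnemySight progress bar through the T_Sight timeline, and StopDetection reverses it.
; A full bar sends the chase message, while an emptied bar hides after a short delay and sends stop-chase.
; Tick turns the widget toward the player camera; Damage only prints debug text.
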(event EventStartDetection
  (params (AI :type BP%20Enemy%20Controller%20Object%20Reference))
  (bind _sight_progress_bar (Variables|Default|GetSight%20Progress%20Bar))
  ;[1 1 1] Event Function - Fill / Empty the Sight Widget
  (Widget|SetVisibility _sight_progress_bar "Visible")
  (bind (_direction _sight_alpha) (Timeline|T_Sight Play)
    (:Update
      (Progress|SetPercent _sight_progress_bar _sight_alpha)
      (Development|PrintString (Utilities|String|ToString(Float) _sight_alpha)))
    (:Finished
      (switch Utilities|FlowControl|Switch|SwitchonETimelineDirection _direction
        (:Forward
          (Class|BPIAlertSystem|StartChase(Message) AI))
        (:Backward
          (Utilities|FlowControl|RetriggerableDelay 0.5)
          (Widget|SetVisibility _sight_progress_bar "Hidden")
          (Class|BPIAlertSystem|StopChase(Message) AI))))))

(event EventStopDetection
  (bind _sight_progress_bar (Variables|Default|GetSight%20Progress%20Bar))
  ;[1 1 1] Event Function - Fill / Empty the Sight Widget
  (bind (_direction _sight_alpha) (Timeline|T_Sight Reverse)
    (:Update
      (Progress|SetPercent _sight_progress_bar _sight_alpha)
      (Development|PrintString (Utilities|String|ToString(Float) _sight_alpha)))
    (:Finished
      (switch Utilities|FlowControl|Switch|SwitchonETimelineDirection _direction
        (:Forward
          (Class|BPIAlertSystem|StartChase(Message) (stale EventStartDetection AI)))
        (:Backward
          (Utilities|FlowControl|RetriggerableDelay 0.5)
          (Widget|SetVisibility _sight_progress_bar "Hidden")
          (Class|BPIAlertSystem|StopChase(Message) (stale EventStartDetection AI)))))))

(event EventTick
  (params (DeltaSeconds :type Float%20%28single-precision%29))
  (bind _widget (Variables|Default|GetWidget))
  ;[1 1 1] Event Tick - Rotate Sight Bar
  (Transformation|SetWorldRotation _widget (Math|Rotator|FindLookatRotation (Transformation|GetWorldLocation _widget) (Transformation|GetWorldLocation (Variables|/Script/Engine.Actor|GetRootComponent (Game|GetPlayerCameraManager 0)))) false false))

(event EventBeginPlay
  ;[1 1 1] Event Begin Play - Set Widget Sight Bar
  (bind _aswd_enemy_sight (Utilities|Casting|CastToWD_EnemySight (UserInterface|GetWidget (Variables|Default|GetWidget))))
  (Variables|Default|SetSight%20Progress%20Bar (Variables|/Game/Enemy/WD_EnemySight.WD_EnemySight_C|GetSight_ProgressBar _aswd_enemy_sight)))

(event EventDamage
  (Development|PrintString "TOMEI DAMAGE"))

(fn ConstructionScript)