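; BP_ButtonSwitch is an interactable button that opens a BP_Door when E is pressed.
; On BeginPlay it caches the door found by GetActorOfClass, with no per-instance link.
; A Player-tagged actor overlapping its Trigger enables input on the button, and nothing disables it afterward.
; Pressing E shows the TextRender, sets the door's ButtonPressed flag, prints it and calls OpenDoor.
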(event OnComponentBeginOverlap(Trigger)
  (params (OverlappedComponent :type Primitive%20Component%20Object%20Reference) (OtherActor :type Actor%20Object%20Reference) (OtherComp :type Primitive%20Component%20Object%20Reference) (OtherBodyIndex :type Integer) (bFromSweep :type Boolean) (SweepResult :type Hit%20Result%20Structure%20%28by%20ref%29))
  (if (Actor|ActorHasTag OtherActor "Player")
    (Input|EnableInput (Game|GetPlayerController 0))))

(event EventBeginPlay
  (bind _returnvalue (Actor|GetActorOfClass "/Game/Interactables/BP_Door.BP_Door_C"))
  (Variables|Default|SetMrDoor _returnvalue))

(event Input|KeyboardEvents|E
  (params (Key :type Key%20Structure :default "None"))
  (bind _mrdoor (Variables|Default|GetMrDoor))
  (:Pressed
    (Rendering|SetVisibility (Variables|Default|GetTextRender) true false)
    (bind _output_get (Variables|/Game/Interactables/BP_Door.BP_Door_C|SetButtonPressed _mrdoor true))
    (Development|PrintString (Utilities|String|ToString(Boolean) _output_get))
    (Default|OpenDoor _mrdoor)))

(fn ConstructionScript)