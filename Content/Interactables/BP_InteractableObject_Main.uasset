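; BP_InteractableObject_Main is an interactable object whose cube trigger reacts when hit by an actor tagged Shuriken.
; An enum state selects the reaction: destroy the cube component, play a 2D explosion sound, or briefly enable physics.
; The physics reaction switches the cube to Movable and simulates physics, then sets mobility back to Static after a short delay.
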(event OnComponentHit(CubeTrigger)
  (params (HitComponent :type Primitive%20Component%20Object%20Reference) (OtherActor :type Actor%20Object%20Reference) (OtherComp :type Primitive%20Component%20Object%20Reference) (NormalImpulse :type Vector :default "0, 0, 0") (Hit :type Hit%20Result%20Structure%20%28by%20ref%29))
  (bind _cubetrigger (Variables|Default|GetCubeTrigger))
  (if (Actor|ActorHasTag OtherActor "Shuriken")
    (switch Utilities|FlowControl|Switch|SwitchonEN_InteractablesStates (Variables|Default|GetEnumStates)
      (:NewEnumerator0
        (Components|DestroyComponent (Variables|Default|GetCubeTrigger)))
      (:NewEnumerator1
        (Audio|PlaySound2D "/Game/StarterContent/Audio/Explosion01.Explosion01" 1.0 1.0 0.0 0 0))
      (:NewEnumerator2
        (Transformation|SetMobility _cubetrigger "Movable")
        (Physics|SetSimulatePhysics _cubetrigger true)
        (Utilities|FlowControl|Delay 1.0)
        (Transformation|SetMobility _cubetrigger "Static")))))

(fn ConstructionScript)