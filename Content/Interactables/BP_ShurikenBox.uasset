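; BP_ShurikenBox is a pickup that adds three shurikens to the player's current count.
; When a Player-tagged actor enters its trigger, a DoOnce gate limits it to one award, made through a cast to BP_ThirdPersonCharacter.
; It then plays the ring-collected sound at the trigger's location and destroys itself after a short delay.
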(event OnComponentBeginOverlap(Trigger)
  (params (OverlappedComponent :type Primitive%20Component%20Object%20Reference) (OtherActor :type Actor%20Object%20Reference) (OtherComp :type Primitive%20Component%20Object%20Reference) (OtherBodyIndex :type Integer) (bFromSweep :type Boolean) (SweepResult :type Hit%20Result%20Structure%20%28by%20ref%29))
  (if (Actor|ActorHasTag OtherActor "Player")
    (Utilities|FlowControl|DoOnce false
      (:Completed
        (bind _asbp_third_person_character (Utilities|Casting|CastToBP_ThirdPersonCharacter OtherActor))
        (Variables|/Game/ThirdPerson/Blueprints/BP_ThirdPersonCharacter.BP_ThirdPersonCharacter_C|SetShurikenCurrent _asbp_third_person_character (+ (Variables|/Game/ThirdPerson/Blueprints/BP_ThirdPersonCharacter.BP_ThirdPersonCharacter_C|GetShurikenCurrent _asbp_third_person_character) 3))
        (Audio|PlaySoundatLocation "/Game/SFX/SC_RingCollected.SC_RingCollected" (Transformation|GetWorldLocation (Variables|Default|GetTrigger)) "0, 0, 0" 1.0 1.0 0.0 0 0 0 0)
        (Utilities|FlowControl|Delay 0.2)
        (Actor|DestroyActor)))))

(fn ConstructionScript)